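; Enemy Blueprint that chases the player character when it sees it and can be destroyed by damage.
; PawnSensing sightings that cast to ThirdPersonCharacter trigger AI MoveTo with that character as target actor and player 0's location as destination.
; Any damage sets Health to damage minus current Health, a reversed subtraction, and destroys the actor at zero or below.
; A Health debug print is left unconnected.
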(event `self.PawnSensing.OnSeePawn`
  (params (Pawn :type "Pawn Object Reference"))
  (bind _asthird_person_character (cast `/Game/ThirdPersonBP/Blueprints/ThirdPersonCharacter` Pawn))
  (`|AIMoveTo` self (`self.K2_GetActorLocation` (`GameplayStatics.GetPlayerCharacter` 0)) _asthird_person_character))

(event `self.ReceiveAnyDamage`
  (params (Damage :type "Float (single-precision)") (DamageType :type "DamageType Object Reference") (InstigatedBy :type "Controller Object Reference") (DamageCauser :type "Actor Object Reference"))
  (bind _output_get (set `self.Health` (- Damage (`self.Health`))))
  (if (<= _output_get 0.0)
    (`self.K2_DestroyActor`)))

(fn `UserConstructionScript`)