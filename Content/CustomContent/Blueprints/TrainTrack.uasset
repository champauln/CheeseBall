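; TrainTrack is a pickup actor that gives the overlapping ThirdPersonCharacter a train track when Left Shift is pressed.
; It enables input for player controller 0 on BeginPlay, and its Box overlap opens and closes a Gate that filters the key press.
; A pickup zeroes then increments the character's TrainTracksHeld, leaving it at one, prints a message and destroys the actor.
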(event `self.ReceiveBeginPlay`
  (`self.EnableInput` (`GameplayStatics.GetPlayerController` 0)))

(event `Key|LeftShift` :consume false
  (params (Key :type "Key Structure" :default "AnyKey"))
  (:`Pressed`
    (`/Engine/EditorBlueprintResources/StandardMacros.Gate` true :!label _label
      (:`Exit`
        (bind _output_get (set `/Game/CustomContent/Blueprints/ThirdPersonCharacter.TrainTracksHeld` 0 (stale `self.Box.OnComponentBeginOverlap` _asthird_person_character)))
        (`/Engine/EditorBlueprintResources/StandardMacros.IncrementInt` _output_get
          (:`  `
            (`KismetSystemLibrary.PrintString` "Track got")
            (`self.K2_DestroyActor`)))))))

(event `self.Box.OnComponentBeginOverlap`
  (params (OverlappedComponent :type "PrimitiveComponent Object Reference") (OtherActor :type "Actor Object Reference") (OtherComp :type "PrimitiveComponent Object Reference") (OtherBodyIndex :type Integer) (bFromSweep :type Boolean) (SweepResult :type "HitResult Structure (by ref)"))
  (bind _asthird_person_character (cast `/Game/CustomContent/Blueprints/ThirdPersonCharacter` OtherActor))
  (goto _label :!via `Open`))

(event `self.Box.OnComponentEndOverlap`
  (params (OverlappedComponent :type "PrimitiveComponent Object Reference") (OtherActor :type "Actor Object Reference") (OtherComp :type "PrimitiveComponent Object Reference") (OtherBodyIndex :type Integer))
  (goto _label :!via `Close`))

(fn `UserConstructionScript`)