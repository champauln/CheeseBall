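; BOSSBOT is a boss actor that counts hits and plays a staged explosion sequence when its health runs out.
; AnyDamage subtracts one HEALTH per damage event, regardless of the damage amount.
; At zero or below, it spawns scaled-up explosion Blueprints at Sphere, Sphere1 and StaticMesh, separated by Delays, with the last one largest.
; The graph does not destroy the actor or guard the sequence against further damage.
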(event `self.ReceiveAnyDamage`
  (params (Damage :type "Float (single-precision)") (DamageType :type "DamageType Object Reference") (InstigatedBy :type "Controller Object Reference") (DamageCauser :type "Actor Object Reference"))
  (bind _output_get (set `self.HEALTH` (- (`self.HEALTH`) 1.0)))
  (if (<= _output_get 0.0)
    (bind _returnvalue (`|SpawnActorFromClass` "/Game/CustomContent/Particles/P_Explosion_Blueprint.P_Explosion_Blueprint_C" (`KismetMathLibrary.Conv_VectorToTransform` (`SceneComponent.K2_GetComponentLocation` (`self.Sphere`))) "Undefined" "OverrideRootScale"))
    (`self.SetActorScale3D` _returnvalue (`KismetMathLibrary.MakeVector` 3.0 3.0 3.0))
    (`KismetSystemLibrary.Delay` 1.0)
    (bind _returnvalue_2 (`|SpawnActorFromClass` "/Game/CustomContent/Particles/P_Explosion_Blueprint.P_Explosion_Blueprint_C" (`KismetMathLibrary.Conv_VectorToTransform` (`SceneComponent.K2_GetComponentLocation` (`self.Sphere1`))) "Undefined" "OverrideRootScale"))
    (`self.SetActorScale3D` _returnvalue_2 (`KismetMathLibrary.MakeVector` 3.0 3.0 3.0))
    (`KismetSystemLibrary.Delay` 1.0)
    (bind _returnvalue_3 (`|SpawnActorFromClass` "/Game/CustomContent/Particles/P_Explosion_Blueprint.P_Explosion_Blueprint_C" (`KismetMathLibrary.Conv_VectorToTransform` (`SceneComponent.K2_GetComponentLocation` (`self.StaticMesh`))) "Undefined" "OverrideRootScale"))
    (`self.SetActorScale3D` _returnvalue_3 (`KismetMathLibrary.MakeVector` 10.0 10.0 10.0))))

(fn `UserConstructionScript`)