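; Ammo pickup actor that tops up the player's ammo when walked over.
; On Tick it steps a degree counter to spin around yaw at a fixed roll tilt, so spin speed depends on frame rate.
; When the player character overlaps it, it casts to ThirdPersonCharacter, adds a fixed amount to AmmoCount up to a cap, then destroys itself.
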(event `self.ReceiveTick`
  (params (DeltaSeconds :type "Float (single-precision)"))
  (bind _deg (`self.DEG`))
  (`self.K2_SetActorRotation` (struct))
  (bind _result (`/Engine/EditorBlueprintResources/StandardMacros.IncrementInt` _deg)
    (:`  `
      (if (== _deg 359)
        (set `self.DEG` 0))
      (`self.K2_SetActorRotation` (`KismetMathLibrary.MakeRotator` 45.0 0.0 (`KismetMathLibrary.Conv_IntToDouble` _result))))))

(event `self.ReceiveActorBeginOverlap`
  (params (OtherActor :type "Actor Object Reference"))
  (bind _returnvalue (`GameplayStatics.GetPlayerCharacter` 0))
  (if (== OtherActor _returnvalue)
    (bind _asthird_person_character (cast `/Game/CustomContent/Blueprints/ThirdPersonCharacter` _returnvalue))
    (bind _ammocount (`/Game/CustomContent/Blueprints/ThirdPersonCharacter.AmmoCount` _asthird_person_character))
    (set `/Game/CustomContent/Blueprints/ThirdPersonCharacter.AmmoCount` (+ 10 _ammocount) _asthird_person_character)
    (if (>= _ammocount 100)
      (set `/Game/CustomContent/Blueprints/ThirdPersonCharacter.AmmoCount` 100 _asthird_person_character))
    (`self.K2_DestroyActor`)))

(fn `UserConstructionScript`)