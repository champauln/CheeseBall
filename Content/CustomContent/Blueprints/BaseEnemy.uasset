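; BaseEnemy is an enemy pawn that chases the player and self-destructs on contact.
; Tick moves it toward the player with SimpleMoveToActor and turns its capsule to face them; the PawnSensing event is empty.
; Overlapping the player applies damage, spawns an explosion and ammo pickup, then destroys the enemy.
; Incoming damage reduces and prints Health; death randomly drops ammo, health or nothing.
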(event `self.ReceiveActorBeginOverlap`
  (params (OtherActor :type "Actor Object Reference"))
  (bind _returnvalue (`GameplayStatics.GetPlayerCharacter` 0))
  (bind _returnvalue_2 (`self.GetTransform`))
  (if (== OtherActor _returnvalue)
    (`GameplayStatics.ApplyDamage` _returnvalue 0.1)
    (`|SpawnActorFromClass` "/Game/CustomContent/Particles/P_Explosion_Blueprint.P_Explosion_Blueprint_C" _returnvalue_2 "Undefined" "OverrideRootScale")
    (`|SpawnActorFromClass` "/Game/CustomContent/Blueprints/AmmoPickup.AmmoPickup_C" _returnvalue_2 "Undefined" "OverrideRootScale")
    (`self.K2_DestroyActor`)))

(event `self.ReceiveTick`
  (params (DeltaSeconds :type "Float (single-precision)"))
  (`NavigationSystem.SimpleMoveToActor` (`self.GetController`) (`GameplayStatics.GetPlayerPawn` 0))
  (`SceneComponent.K2_SetRelativeRotation` (`self.CapsuleComponent`) (`KismetMathLibrary.FindLookAtRotation` (`self.K2_GetActorLocation`) (`self.K2_GetActorLocation` (`GameplayStatics.GetPlayerCharacter` 0))) false false))

(event `self.PawnSensing.OnSeePawn`
  (params (Pawn :type "Pawn Object Reference")))

(event `self.ReceiveAnyDamage`
  (params (Damage :type "Float (single-precision)") (DamageType :type "DamageType Object Reference") (InstigatedBy :type "Controller Object Reference") (DamageCauser :type "Actor Object Reference"))
  (bind _returnvalue (`KismetMathLibrary.Conv_VectorToTransform` (`self.K2_GetActorLocation`)))
  (bind _output_get (set `self.Health` (- (`self.Health`) Damage)))
  (`KismetSystemLibrary.PrintString` (`KismetStringLibrary.Conv_DoubleToString` _output_get))
  (if (<= _output_get 0.0)
    (switch `int` (`KismetMathLibrary.RandomInteger` 3)
      (:`0`
        _)
      (:`1`
        (`|SpawnActorFromClass` "/Game/CustomContent/Blueprints/AmmoPickup.AmmoPickup_C" _returnvalue "Undefined" "OverrideRootScale"))
      (:`2`
        (`|SpawnActorFromClass` "/Game/CustomContent/Blueprints/HealthPickup.HealthPickup_C" _returnvalue "Undefined" "OverrideRootScale")))
    (`self.K2_DestroyActor`)))

(fn `UserConstructionScript`)