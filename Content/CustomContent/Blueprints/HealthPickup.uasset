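; Health pickup actor that restores part of the player's health on overlap, then destroys itself.
; Tick spins the actor by advancing an integer yaw counter one degree per frame and wrapping it, so spin speed depends on frame rate.
; Overlap reacts only to player character 0, cast to ThirdPersonCharacter, adding a quarter to its normalized PlayerHealth and capping it at full.
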(event `self.ReceiveTick`
  (params (DeltaSeconds :type "Float (single-precision)"))
  (bind _deg (`self.DEG`))
  (`self.K2_SetActorRotation` (struct))
  (bind _result (`/Engine/EditorBlueprintResources/StandardMacros.IncrementInt` _deg)
    (:`  `
      (if (== _deg 359)
        (set `self.DEG` 0))
      (`self.K2_SetActorRotation` (`KismetMathLibrary.MakeRotator` 0.0 0.0 (`KismetMathLibrary.Conv_IntToDouble` _result))))))

(event `self.ReceiveActorBeginOverlap`
  (params (OtherActor :type "Actor Object Reference"))
  (bind _returnvalue (`GameplayStatics.GetPlayerCharacter` 0))
  (if (== OtherActor _returnvalue)
    (bind _asthird_person_character (cast `/Game/CustomContent/Blueprints/ThirdPersonCharacter` _returnvalue))
    (bind _playerhealth (`/Game/CustomContent/Blueprints/ThirdPersonCharacter.PlayerHealth` _asthird_person_character))
    (set `/Game/CustomContent/Blueprints/ThirdPersonCharacter.PlayerHealth` (+ _playerhealth 0.25) _asthird_person_character)
    (if (>= _playerhealth 1.0)
      (set `/Game/CustomContent/Blueprints/ThirdPersonCharacter.PlayerHealth` 1.0 _asthird_person_character))
    (`self.K2_DestroyActor`)))

(fn `UserConstructionScript`)